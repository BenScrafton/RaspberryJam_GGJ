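; Two-sided store shelf actor that holds grocery items and flings them off when hit by a character pawn.
; Initialise caches spawn-point locations, then SpawnItems fills both sides with one item type from a data table.
; Each side fires once, when the pawn's CanRam is false, applying impulses along the hit normal with upward bias, negated on side two.
; DespawnRandomItems removes items randomly from either side.
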(event OnComponentHit(Shelf_01)
  (params (HitComponent :type Primitive%20Component%20Object%20Reference) (OtherActor :type Actor%20Object%20Reference) (OtherComp :type Primitive%20Component%20Object%20Reference) (NormalImpulse :type Vector :default "0, 0, 0") (Hit :type Hit%20Result%20Structure%20%28by%20ref%29))
  (if (not (Variables|Default|GethasProjectedItems01))
    (bind _asbp_character_pawn (Utilities|Casting|CastToBP_CharacterPawn OtherActor))
    (if (not (Variables|/Game/Blueprints/Character/BP_CharacterPawn.BP_CharacterPawn_C|GetcanRam _asbp_character_pawn))
      (CallFunction|ProjectItems (Variables|Default|GetItems01) (* (+ (.normal Hit) "0.000000,0.000000,0.300000") (Math|Float|MakeLiteralFloat 1.0)))
      (Variables|Default|SethasProjectedItems01 true))))

(event OnComponentHit(Shelf_02)
  (params (HitComponent :type Primitive%20Component%20Object%20Reference) (OtherActor :type Actor%20Object%20Reference) (OtherComp :type Primitive%20Component%20Object%20Reference) (NormalImpulse :type Vector :default "0, 0, 0") (Hit :type Hit%20Result%20Structure%20%28by%20ref%29))
  (if (not (Variables|Default|GethasProjectedItems02))
    (bind _asbp_character_pawn (Utilities|Casting|CastToBP_CharacterPawn OtherActor))
    (if (not (Variables|/Game/Blueprints/Character/BP_CharacterPawn.BP_CharacterPawn_C|GetcanRam _asbp_character_pawn))
      (Development|PrintString "Hello")
      (CallFunction|ProjectItems (Variables|Default|GetItems02) (* (+ (.normal Hit) "0.000000,0.000000,0.300000") (Math|Float|MakeLiteralFloat -1.0)))
      (Variables|Default|SethasProjectedItems02 true))))

(event EventBeginPlay)

(event Collision|EventActorBeginOverlap
  (params (OtherActor :type Actor%20Object%20Reference)))

(event EventTick
  (params (DeltaSeconds :type Float%20%28single-precision%29)))

(fn ConstructionScript)

(fn SpawnItems
  (params (ItemTypes :type ItemType%20Enum :default "NewEnumerator0"))
  (Utilities|FlowControl|Sequence
    (:then_0
      (switch Utilities|FlowControl|Switch|SwitchonItemType ItemTypes
        (:NewEnumerator0
          (Variables|Default|Setrowname "Can"))
        (:NewEnumerator1
          (Variables|Default|Setrowname "Milk"))
        (:NewEnumerator2
          (Variables|Default|Setrowname "Eggs"))
        (:NewEnumerator3
          (Variables|Default|Setrowname "Bread"))
        (:NewEnumerator4
          (Variables|Default|Setrowname "Meat"))
        (:NewEnumerator5
          (Variables|Default|Setrowname "Banana"))))
    (:then_1
      (if (Variables|Default|GetisInitialised)
        (bind _returnvalue (Utilities|GetDataTableRow "/Game/Blueprints/Items/Generic/ItemsDataTable.ItemsDataTable" (Variables|Default|Getrowname))
          (:then
            (Variables|Default|SetItemTypeStored (.type _returnvalue))
            (Variables|Default|SetItemMesh (.mesh _returnvalue))
            (for _array_element (Variables|Default|GetItemSpawnPoints01)
              (bind _returnvalue_2 (Game|SpawnActorfromClass "/Game/Blueprints/Items/Generic/Item.Item_C" (Math|Transform|MakeTransform _array_element "0, 0, 0" (.scalefactor _returnvalue)) "Undefined" "MultiplyWithRoot" 0 0))
              (Default|Initialise _returnvalue_2 (Variables|Default|GetItemTypeStored) (Variables|Default|GetItemMesh))
              (Utilities|Array|Add (Variables|Default|GetItems01) _returnvalue_2))
            (for _array_element_2 (Variables|Default|GetItemSpawnPoints02)
              (bind _returnvalue_3 (Game|SpawnActorfromClass "/Game/Blueprints/Items/Generic/Item.Item_C" (Math|Transform|MakeTransform _array_element_2 "0, 0, 0" (.scalefactor _returnvalue)) "Undefined" "MultiplyWithRoot" 0 0))
              (Default|Initialise _returnvalue_3 (Variables|Default|GetItemTypeStored) (Variables|Default|GetItemMesh))
              (Utilities|Array|Add (Variables|Default|GetItems02) _returnvalue_3))))))
    (:then_2
      (Development|PrintString (Utilities|String|ToString(Integer) (Utilities|Array|Length (Variables|Default|GetItems02)))))))

(fn Initialise
  (for _array_element (Components|GetChildrenComponents (Variables|Default|GetItemSpawns01) false)
    (Utilities|Array|Add (Variables|Default|GetItemSpawnPoints01) (Transformation|GetWorldLocation _array_element)))
  (for _array_element_2 (Components|GetChildrenComponents (Variables|Default|GetItemSpawns02) false)
    (Utilities|Array|Add (Variables|Default|GetItemSpawnPoints02) (Transformation|GetWorldLocation _array_element_2)))
  (Variables|Default|SetisInitialised true))

(fn ProjectItems
  (params (items :type Array%20of%20Item%20Object%20References) (direction :type Vector))
  (for _array_element items
    (Utilities|IsValid _array_element
      (:Is%20Valid
        (Physics|AddImpulse (Variables|/Game/Blueprints/Items/Generic/Item.Item_C|GetItemModel _array_element) (* direction (Variables|Default|GetProjectionForce)) "None" false)))))

(fn DespawnRandomItems
  (params (numDespawn :type Integer))
  (Development|PrintString (Utilities|String|ToString(Integer) (Utilities|Array|Length (Variables|Default|GetItems01))))
  (for _index (range 0 numDespawn)
    (if (Math|Random|RandomBool)
      (Utilities|Array|RemoveItem (Variables|Default|GetItems01) (Utilities|Array|Get(acopy) (Variables|Default|GetItems01) _index))
      (Utilities|IsValid (Utilities|Array|Get(acopy) (Variables|Default|GetItems01) _index)
        (:Is%20Valid
          (Actor|DestroyActor (Utilities|Array|Get(acopy) (Variables|Default|GetItems01) _index))))
      (else
        (Utilities|Array|RemoveItem (Variables|Default|GetItems02) (Utilities|Array|Get(acopy) (Variables|Default|GetItems02) _index))
        (Utilities|IsValid (Utilities|Array|Get(acopy) (Variables|Default|GetItems02) _index)
          (:Is%20Valid
            (Actor|DestroyActor (Utilities|Array|Get(acopy) (Variables|Default|GetItems02) _index))))))))