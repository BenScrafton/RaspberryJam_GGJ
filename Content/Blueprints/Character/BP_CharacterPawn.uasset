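; BP_CharacterPawn is a physics-driven character pawn that moves and steers a Trolley component.
; ProcessAcceleration pushes the trolley along its forward vector, scaled by direction and AccelerationFactor, and prints that force for debugging.
; ProcessTurn applies yaw torque scaled by direction and TurnFactor.
; The event graph and construction script are empty, so both functions rely on external callers.
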(event EventBeginPlay)

(event Collision|EventActorBeginOverlap
  (params (OtherActor :type Actor%20Object%20Reference)))

(event EventTick
  (params (DeltaSeconds :type Float%20%28single-precision%29)))

(fn ConstructionScript)

(fn ProcessAcceleration
  (params (Direction :type Float%20%28double-precision%29))
  (bind _accelerationfactor (Variables|Default|GetAccelerationFactor))
  (bind _trolley (Variables|Default|GetTrolley))
  (bind _returnvalue (Math|Vector|GetForwardVector _trolley))
  (bind _returnvalue_2 (* _accelerationfactor Direction _returnvalue))
  (Physics|AddForce (Variables|Default|Gettrolley) _returnvalue_2 "None" false)
  (Development|PrintString (Utilities|String|ToString(Vector) _returnvalue_2)))

(fn ProcessTurn
  (params (Direction :type Float%20%28double-precision%29))
  (Class|PrimitiveComponent|AddTorqueinDegrees (Variables|Default|GetTrolley) (Math|Vector|MakeVector 0.0 0.0 (* (Variables|Default|GetTurnFactor) Direction)) "None" false))