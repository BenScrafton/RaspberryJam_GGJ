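; BP_Player_Controller is the player controller that routes Enhanced Input to the player's BP_CharacterPawn.
; On BeginPlay it adds PlayerInputMapping to the local player's input subsystem.
; The accelerate and turn actions cast player pawn 0 to BP_CharacterPawn and pass their values to its ProcessAcceleration and ProcessTurn functions, leaving movement logic to the pawn.
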(event Input|EnhancedActionEvents|EnhancedInputActionActionPlayerAccelerate
  (params (ActionValue :type Float%20%28double-precision%29) (ElapsedSeconds :type Float%20%28double-precision%29) (TriggeredSeconds :type Float%20%28double-precision%29) (InputAction :type Input%20Action%20Object%20Reference :default "/Game/Blueprints/Input/ActionPlayerAccelerate.ActionPlayerAccelerate"))
  (:Triggered
    (bind _asbp_character_pawn (Utilities|Casting|CastToBP_CharacterPawn (Game|Player|GetPlayerPawn 0)))
    (Default|ProcessAcceleration _asbp_character_pawn ActionValue)))

(event Input|EnhancedActionEvents|EnhancedInputActionActionPlayerTurn
  (params (ActionValue :type Float%20%28double-precision%29) (ElapsedSeconds :type Float%20%28double-precision%29) (TriggeredSeconds :type Float%20%28double-precision%29) (InputAction :type Input%20Action%20Object%20Reference :default "/Game/Blueprints/Input/ActionPlayerTurn.ActionPlayerTurn"))
  (:Triggered
    (bind _asbp_character_pawn (Utilities|Casting|CastToBP_CharacterPawn (Game|Player|GetPlayerPawn 0)))
    (Default|ProcessTurn _asbp_character_pawn ActionValue)))

(event EventBeginPlay
  (Input|AddMappingContext (PlayerController|LocalPlayerSubsystems|GetEnhancedInputLocalPlayerSubsystem (Game|GetPlayerController 0)) "/Game/Blueprints/Input/PlayerInputMapping.PlayerInputMapping" 0 "(bIgnoreAllPressedKeysUntilRelease=True,bForceImmediately=False)"))

(fn ConstructionScript)